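; Grid board actor for LaserLab that lays out a puzzle level of blocks and four mirror orientations.
; The construction script rebuilds instanced floor tiles and pieces from the flattened Cells array, plus border walls with entry and exit markers at chosen rows.
; BeginPlay makes the board the view target and enables mouse input.
; Tick snaps the cursor hit to a cell in local space and shows a highlight there.
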(event EventBeginPlay
  (bind _returnvalue (Game|GetPlayerController 0))
  (|CallParentFunction)
  (Game|Player|SetViewTargetwithBlend _returnvalue self 0.0 "VTBlend_Linear" 0.0 false)
  (Variables|/Script/Engine.PlayerController|SetbShowMouseCursor _returnvalue true)
  (Variables|/Script/Engine.PlayerController|SetbEnableClickEvents _returnvalue true)
  (Variables|/Script/Engine.PlayerController|SetbEnableMouseOverEvents _returnvalue true)
  (Input|SetInputModeGameandUI _returnvalue 0 (Utilities|Enum|LiteralenumEMouseLockMode "DoNotLock") false false)
  (Rendering|SetVisibility (Variables|Default|GetCellHighlight) false false))

(event Collision|EventActorBeginOverlap
  (params (OtherActor :type Actor%20Object%20Reference)))

(event EventTick
  (params (DeltaSeconds :type Float%20%28single-precision%29))
  (bind _returnvalue (Game|GetPlayerController 0))
  (bind _returnvalue_2 (Transformation|GetActorTransform))
  (bind _returnvalue_3 (Utilities|Enum|LiteralenumETraceTypeQuery "TraceTypeQuery1"))
  (bind _cellsize (Variables|Board|GetCellSize))
  (bind _cellsize_2 (Variables|Board|GetCellSize))
  (bind (_hitresult _returnvalue_4) (Game|Player|GetHitResultUnderCursorbyChannel _returnvalue _returnvalue_3 false))
  (bind (_bblockinghit _binitialoverlap _time _distance _location _impactpoint _normal _impactnormal _physmat _hitactor _hitcomponent) (Collision|BreakHitResult _hitresult))
  (bind _returnvalue_5 (Math|Transform|InverseTransformLocation _returnvalue_2 _location))
  (bind _x (Math|Vector|BreakVector _returnvalue_5))
  (bind _y (Math|Vector|BreakVector _returnvalue_5))
  (bind _returnvalue_6 (/ _x _cellsize))
  (bind _returnvalue_7 (/ _y _cellsize_2))
  (bind _returnvalue_8 (Math|Float|Round _returnvalue_6))
  (bind _returnvalue_9 (Math|Float|Round _returnvalue_7))
  (if _returnvalue_4
    (if (Math|Boolean|ORBoolean (== _hitcomponent (Variables|Default|GetFloorTiles)) (== _hitcomponent (Variables|Default|GetCellHighlight)) (== _hitcomponent (Variables|Default|GetPieces)))
      (if (Math|Boolean|ANDBoolean (>= _returnvalue_8 0) (< _returnvalue_8 (Variables|Board|GetColumns)) (>= _returnvalue_9 0) (< _returnvalue_9 (Variables|Board|GetRows)))
        (Transformation|SetRelativeLocation (Variables|Default|GetCellHighlight) (Math|Vector|MakeVector (* (Math|Conversions|ToFloat(Integer) _returnvalue_8) (Variables|Board|GetCellSize)) (* (Math|Conversions|ToFloat(Integer) _returnvalue_9) (Variables|Board|GetCellSize)) 12.0) false false)
        (Rendering|SetVisibility (Variables|Default|GetCellHighlight) true false)
        (else
          (Rendering|SetVisibility (Variables|Default|GetCellHighlight) false false)))
      (else
        (Rendering|SetVisibility (Variables|Default|GetCellHighlight) false false)))
    (else
      (Rendering|SetVisibility (Variables|Default|GetCellHighlight) false false))))

(fn ConstructionScript
  (bind _cellsize (Variables|Board|GetCellSize))
  (bind _columns (Variables|Board|GetColumns))
  (bind _cellsize_2 (Variables|Board|GetCellSize))
  (bind _returnvalue (Math|Conversions|ToFloat(Integer) _columns))
  (bind _returnvalue_2 (* -1.0 _cellsize))
  (bind _returnvalue_3 (* _returnvalue _cellsize_2))
  (Utilities|Array|Resize (Variables|Board|GetCells) (* (Variables|Board|GetRows) (Variables|Board|GetColumns)))
  (Components|InstancedStaticMesh|ClearInstances (Variables|Default|GetFloorTiles))
  (Components|InstancedStaticMesh|ClearInstances (Variables|Default|GetWalls))
  (Components|InstancedStaticMesh|ClearInstances (Variables|Default|GetEntryMarker))
  (Components|InstancedStaticMesh|ClearInstances (Variables|Default|GetEndpointMarker))
  (Components|InstancedStaticMesh|ClearInstances (Variables|Default|GetPieces))
  (for _index (range 0 (- (Variables|Board|GetRows) 1))
    (for _index_2 (range 0 (- (Variables|Board|GetColumns) 1))
      (Components|InstancedStaticMesh|AddInstance (Variables|Default|GetFloorTiles) (Math|Transform|MakeTransform (Math|Vector|MakeVector (* (Math|Conversions|ToFloat(Integer) _index_2) (Variables|Board|GetCellSize)) (* (Math|Conversions|ToFloat(Integer) _index) (Variables|Board|GetCellSize)) 4.0) "0.0,0.0,0.0" "0.92,0.92,0.08") false)
      ;[0.15 0.15 0.15 0.5] NewEnumerator4 Empty, NewEnumerator5 Block, NewEnumerator0 MirrorNE, NewEnumerator1 MirrorNW, NewEnumerator2 MirrorSE, NewEnumerator3 MirrorSW
      (switch Utilities|FlowControl|Switch|SwitchonECellState (Utilities|Array|Get(acopy) (Variables|Board|GetCells) (+ (* _index (Variables|Board|GetColumns)) _index_2))
        (:NewEnumerator5
          (Components|InstancedStaticMesh|AddInstance (Variables|Default|GetPieces) (Math|Transform|MakeTransform (Math|Vector|MakeVector (* (Math|Conversions|ToFloat(Integer) _index_2) (Variables|Board|GetCellSize)) (* (Math|Conversions|ToFloat(Integer) _index) (Variables|Board|GetCellSize)) 45.0) "0.0,0.0,0.0" "0.7,0.7,0.7") false))
        (:NewEnumerator0
          (Components|InstancedStaticMesh|AddInstance (Variables|Default|GetPieces) (Math|Transform|MakeTransform (Math|Vector|MakeVector (* (Math|Conversions|ToFloat(Integer) _index_2) (Variables|Board|GetCellSize)) (* (Math|Conversions|ToFloat(Integer) _index) (Variables|Board|GetCellSize)) 3e+01) "0.0,45.0,0.0" "0.9,0.12,0.5") false))
        (:NewEnumerator1
          (Components|InstancedStaticMesh|AddInstance (Variables|Default|GetPieces) (Math|Transform|MakeTransform (Math|Vector|MakeVector (* (Math|Conversions|ToFloat(Integer) _index_2) (Variables|Board|GetCellSize)) (* (Math|Conversions|ToFloat(Integer) _index) (Variables|Board|GetCellSize)) 3e+01) "0.0,-45.0,0.0" "0.9,0.12,0.5") false))
        (:NewEnumerator2
          (Components|InstancedStaticMesh|AddInstance (Variables|Default|GetPieces) (Math|Transform|MakeTransform (Math|Vector|MakeVector (* (Math|Conversions|ToFloat(Integer) _index_2) (Variables|Board|GetCellSize)) (* (Math|Conversions|ToFloat(Integer) _index) (Variables|Board|GetCellSize)) 3e+01) "0.0,135.0,0.0" "0.9,0.12,0.5") false))
        (:NewEnumerator3
          (Components|InstancedStaticMesh|AddInstance (Variables|Default|GetPieces) (Math|Transform|MakeTransform (Math|Vector|MakeVector (* (Math|Conversions|ToFloat(Integer) _index_2) (Variables|Board|GetCellSize)) (* (Math|Conversions|ToFloat(Integer) _index) (Variables|Board|GetCellSize)) 3e+01) "0.0,-135.0,0.0" "0.9,0.12,0.5") false)))))
  (for _index_3 (range -1 (- (+ (Variables|Board|GetColumns) 1) 1))
    (Components|InstancedStaticMesh|AddInstance (Variables|Default|GetWalls) (Math|Transform|MakeTransform (Math|Vector|MakeVector (* (Math|Conversions|ToFloat(Integer) _index_3) (Variables|Board|GetCellSize)) (* -1.0 (Variables|Board|GetCellSize)) 4e+01) "0.0,0.0,0.0" "0.95,0.95,0.7") false)
    (Components|InstancedStaticMesh|AddInstance (Variables|Default|GetWalls) (Math|Transform|MakeTransform (Math|Vector|MakeVector (* (Math|Conversions|ToFloat(Integer) _index_3) (Variables|Board|GetCellSize)) (* (Math|Conversions|ToFloat(Integer) (Variables|Board|GetRows)) (Variables|Board|GetCellSize)) 4e+01) "0.0,0.0,0.0" "0.95,0.95,0.7") false))
  (for _index_4 (range 0 (- (Variables|Board|GetRows) 1))
    (if (== _index_4 (Variables|Board|GetEntryRow))
      (Components|InstancedStaticMesh|AddInstance (Variables|Default|GetEntryMarker) (Math|Transform|MakeTransform (Math|Vector|MakeVector _returnvalue_2 (* (Math|Conversions|ToFloat(Integer) _index_4) (Variables|Board|GetCellSize)) 55.0) "0.0,0.0,0.0" "0.28,0.28,1.0") false)
      (else
        (Components|InstancedStaticMesh|AddInstance (Variables|Default|GetWalls) (Math|Transform|MakeTransform (Math|Vector|MakeVector _returnvalue_2 (* (Math|Conversions|ToFloat(Integer) _index_4) (Variables|Board|GetCellSize)) 4e+01) "0.0,0.0,0.0" "0.95,0.95,0.7") false)))
    (if (== _index_4 (Variables|Board|GetExitRow))
      (Components|InstancedStaticMesh|AddInstance (Variables|Default|GetEndpointMarker) (Math|Transform|MakeTransform (Math|Vector|MakeVector _returnvalue_3 (* (Math|Conversions|ToFloat(Integer) _index_4) (Variables|Board|GetCellSize)) 55.0) "0.0,0.0,0.0" "0.28,0.28,1.0") false)
      (else
        (Components|InstancedStaticMesh|AddInstance (Variables|Default|GetWalls) (Math|Transform|MakeTransform (Math|Vector|MakeVector _returnvalue_3 (* (Math|Conversions|ToFloat(Integer) _index_4) (Variables|Board|GetCellSize)) 4e+01) "0.0,0.0,0.0" "0.95,0.95,0.7") false)))))